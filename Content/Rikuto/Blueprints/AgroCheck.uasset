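; Behavior tree aggro check that lets the Enemy1 AI detect and follow visible targets.
; Each tick, a large sphere trace around the controlled pawn gathers candidate actors, ignoring other BP_Enemy1 actors.
; A Camera-channel line trace tests line of sight to each, writing TargetToFollow and TargetLocation to the blackboard.
; Failed checks clear only TargetToFollow, keeping the last seen location; the last hit processed decides the target.
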(event EventTick
  (params (OwnerActor :type Actor%20Object%20Reference) (DeltaSeconds :type Float%20%28single-precision%29))
  (if (!= (Variables|Default|GetEnemy1_Controller) 0)
    _
    (else
      (bind _asenemy_1_controller (Utilities|Casting|CastToEnemy1_controller OwnerActor))
      (Variables|Default|SetEnemy1_Controller _asenemy_1_controller)))
  (bind _outactors (Actor|GetAllActorsOfClass "/Game/Rikuto/Blueprints/BP_Enemy1.BP_Enemy1_C"))
  (bind _output_get (Variables|Default|SetMyLocation (Transformation|GetActorLocation (Pawn|GetControlledPawn (Variables|Default|GetEnemy1_Controller)))))
  (bind (_outhits _returnvalue) (Collision|MultiSphereTraceForObjects _output_get (+ (Transformation|GetActorLocation (Pawn|GetControlledPawn (Variables|Default|GetEnemy1_Controller))) "0, 0,15.000000") 1.5e+03 (Utilities|Array|MakeArray (Variables|Default|GetDesiredObjectTypes)) false _outactors "None"))
  (if _returnvalue
    (bind _array_element (Utilities|Array|ForEachLoopwithBreak _outhits)
      (:LoopBody
        (bind _outhit (Collision|LineTraceByChannel (Variables|Default|GetMyLocation) (Transformation|GetActorLocation (.HitActor (Collision|BreakHitResult _array_element))) "TraceTypeQuery2" false _outactors "None"))
        (if (== (.HitActor (Collision|BreakHitResult _outhit)) (.HitActor (Collision|BreakHitResult _array_element)))
          (Class|BTFunctionLibrary|SetBlackboardValueasObject (Variables|Default|GetTargetToFollow) (.HitActor (Collision|BreakHitResult _outhit)))
          (AI|BehaviorTree|SetBlackboardValueasVector (Variables|Default|GetTargetLocation) (Transformation|GetActorLocation (.HitActor (Collision|BreakHitResult _outhit))))
          (else
            (Class|BTFunctionLibrary|SetBlackboardValueasObject (Variables|Default|GetTargetToFollow))))))
    (else
      (Class|BTFunctionLibrary|SetBlackboardValueasObject (Variables|Default|GetTargetToFollow)))))