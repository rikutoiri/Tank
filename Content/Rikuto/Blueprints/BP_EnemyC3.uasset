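; Enemy tank that turns toward the player, sweeps its head and fires when a head line trace hits the player.
; Firing has a 3-second cooldown and a two-bullet cap in TankGameState's EnemyBulletArray, indexed by a number parsed from the actor's display name.
; A looping timer stamps caterpillar-track decals on the ground, and a Bullet hit on Body explodes and destroys the tank.
; The Trace function only computes ray spacing and is not called here.
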(event OnComponentHit(Body)
  (params (HitComponent :type Primitive%20Component%20Object%20Reference) (OtherActor :type Actor%20Object%20Reference) (OtherComp :type Primitive%20Component%20Object%20Reference) (NormalImpulse :type Vector :default "0, 0, 0") (Hit :type Hit%20Result%20Structure%20%28by%20ref%29))
  ;[1 1 1] 大破
  (Utilities|Casting|CastToBullet OtherActor)
  (Effects|SpawnEmitteratLocation "/Game/StarterContent/Particles/P_Explosion_2.P_Explosion_2" (Transformation|GetWorldLocation (Variables|Default|GetBody)) "0, 0, 0" "5.000000,5.000000,5.000000")
  (Actor|DestroyActor))

(event Custom|time
  (bind _returnvalue (Transformation|GetActorLocation))
  (bind _outhit (Collision|LineTraceByChannel _returnvalue (+ _returnvalue (* (Transformation|GetActorUpVector) -1e+03)) "TraceTypeQuery1" false 0 "None"))
  (Rendering|Decal|SpawnDecalatLocation "/Game/Rikuto/Materials/CaterpillarFootprints.CaterpillarFootprints" "120.000000,120.000000,120.000000" (.location _outhit) (Math|Rotator|MakeRotator 0.0 -9e+01 (+ (.yaw (Transformation|GetWorldRotation (Variables|Default|GetBody))) 9e+01)) 0.0))

(event Collision|EventActorBeginOverlap
  (params (OtherActor :type Actor%20Object%20Reference)))

(event EventTick
  (params (DeltaSeconds :type Float%20%28single-precision%29))
  (bind _returnvalue (Transformation|GetActorRotation))
  (bind _self self)
  (bind _enemy1_head (Variables|Default|GetEnemy1_Head))
  (bind _returnvalue_2 (Utilities|GetDisplayName _self))
  (bind _returnvalue_3 (Transformation|GetWorldLocation _enemy1_head))
  (bind _returnvalue_4 (Utilities|String|RightChop _returnvalue_2 9))
  (bind _returnvalue_5 (+ _returnvalue_3 "0, 0, 0"))
  (bind _returnvalue_6 (Math|Conversions|ToInteger(Byte) _returnvalue_4))
  (bind _returnvalue_7 (- _returnvalue_6 1))
  (bind _returnvalue_8 (Actor|GetActorOfClass "/Game/Rikuto/Blueprints/TankGameState.TankGameState_C"))
  (if (Variables|/Game/Rikuto/Blueprints/TankGameState.TankGameState_C|GetPlayerAlive _returnvalue_8) ; プレイヤーが生きているか
    (Transformation|SetWorldRotation (Variables|Default|GetStaticMesh) (Math|Interpolation|RInterpTo (Math|Rotator|MakeRotator (.roll _returnvalue) (.pitch _returnvalue) 0.0) (Math|Rotator|MakeRotator 0.0 0.0 (.yaw (Math|Rotator|FindLookatRotation (Transformation|GetActorLocation) (Transformation|GetActorLocation (Variables|Default|GetPlayer))))) (Utilities|Time|GetWorldDeltaSeconds) 0.0) false false) ; プレイヤーを見る
    ;[1 1 1] 首振り
    (bind _float (Timeline|タイムライン_0 Play)
      (:Update
        (Transformation|SetRelativeRotation (Variables|Default|GetEnemy1_Head) (Math|Rotator|MakeRotator 0.0 0.0 _float) false false)
        (bind (_outhit _returnvalue_9) (Collision|LineTraceByChannel _returnvalue_5 (+ _returnvalue_5 (* (Math|Vector|RotateVectorAroundAxis (Math|Vector|GetForwardVector _enemy1_head) (Variables|Default|GetCurrentAngle) "0.000000,0.000000,1.000000") (Variables|Default|GetDistance))) "TraceTypeQuery1" false 0 "ForOneFrame"))
        (if _returnvalue_9 ; プレイヤーTag持っているか
          (if (Actor|ActorHasTag (.HitActor (Collision|BreakHitResult _outhit)) "Player") ; トレースがプレイヤーに当たっているか
            (if (not (Variables|Default|GetIs%20Stop%20Motion)) ; ストップモーション
              (bind _returnvalue_10 (Actor|GetActorOfClass "/Game/Rikuto/Blueprints/TankGameState.TankGameState_C"))
              (if (> 2 (Utilities|Array|Get(acopy) (Variables|/Game/Rikuto/Blueprints/TankGameState.TankGameState_C|GetEnemyBulletArray _returnvalue_10) _returnvalue_7))
                (Utilities|Array|SetArrayElem (Variables|/Game/Rikuto/Blueprints/TankGameState.TankGameState_C|GetEnemyBulletArray _returnvalue_10) _returnvalue_7 (+ (Utilities|Array|Get(acopy) (Variables|/Game/Rikuto/Blueprints/TankGameState.TankGameState_C|GetEnemyBulletArray _returnvalue_10) _returnvalue_7) 1))
                (bind _returnvalue_11 (Game|SpawnActorfromClass "/Game/kaito/Bullet.Bullet_C" (Transformation|GetWorldTransform (Variables|Default|GetArrow1)) "Undefined" 0 0))
                (Utilities|Array|Add (Variables|/Script/Engine.Actor|GetTags _returnvalue_11) (Utilities|String|StringToName (Utilities|String|Append "EnemyBullet" (Utilities|String|ToString(Integer) _returnvalue_7))))
                (Variables|Default|SetIs%20Stop%20Motion true)
                (Utilities|FlowControl|Delay 3.0) ; 0.2秒後
                (Variables|Default|SetIs%20Stop%20Motion false)))))))))

(event EventBeginPlay
  (bind _returnvalue (Actor|GetActorOfClass "/Game/Rikuto/Blueprints/Player.Player_C"))
  (Variables|Default|SetPlayer _returnvalue)
  (Utilities|Time|SetTimerbyEvent (delegate Custom|time) 0.2 true))

(event Input|MouseEvents|RightMouseButton
  (params (Key :type Key%20Structure :default "None"))
  (:Pressed
    (Development|PrintString "Hello" :!label _label))
  (:Released
    (goto _label)))

(event Input|KeyboardEvents|1
  (params (Key :type Key%20Structure :default "None"))
  (:Pressed
    (Development|PrintString "Hello" :!label _label))
  (:Released
    (goto _label)))

(event Input|KeyboardEvents|M
  (params (Key :type Key%20Structure :default "None"))
  (:Pressed
    (Development|PrintString "Hello" :!label _label))
  (:Released
    (goto _label)))

(fn ConstructionScript)

(fn Trace
  (bind _output_get (Variables|Default|SetLast%20Index (Math|Float|Ceil (/ (* (Variables|Default|GetAngle) 2.0) (Variables|Default|GetSpacingAngle))))) ; トレースの数
  (Variables|Default|SetSpacingAngle (/ (* (Variables|Default|GetAngle) 2.0) (Math|Conversions|ToFloat(Integer) _output_get))))