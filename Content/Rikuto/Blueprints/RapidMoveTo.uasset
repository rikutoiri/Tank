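; Behavior tree task that moves an enemy's pawn to the actor stored in the TargetToFollow blackboard key.
; On execute it casts the owner to Enemy1_controller if none is cached, then runs AI MoveTo on the controlled pawn with a small acceptance radius.
; It finishes successfully when the move succeeds, but never calls FinishExecute on a failed move or cast.
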(event EventReceiveExecute
  (params (OwnerActor :type Actor%20Object%20Reference))
  (if (!= (Variables|Default|GetEnemyController) 0)
    _
    (else
      (bind _asenemy_1_controller (Utilities|Casting|CastToEnemy1_controller OwnerActor))
      (Variables|Default|SetEnemyController _asenemy_1_controller)))
  (AI|AIMoveTo (Pawn|GetControlledPawn (Variables|Default|GetEnemyController)) "0, 0, 0" (AI|BehaviorTree|GetBlackboardValueasActor (Variables|Default|GetTargetToFollow)) 5e+01 false
    (:OnSuccess
      (AI|BehaviorTree|FinishExecute true))))