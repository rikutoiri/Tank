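; Enemy tank that hunts the player, leaves timed track decals and explodes when hit by bullets or mines.
; While the player lives, it faces them and swings its head on a timeline, firing when the head's line trace hits them, then pausing.
; KindofTank sets meshes and normal or fast bullets.
; A number parsed from its display name indexes the TankGameState bullet-count cap and tags its shots.
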(event OnComponentHit(Body)
  (params (HitComponent :type Primitive%20Component%20Object%20Reference) (OtherActor :type Actor%20Object%20Reference) (OtherComp :type Primitive%20Component%20Object%20Reference) (NormalImpulse :type Vector :default "0, 0, 0") (Hit :type Hit%20Result%20Structure%20%28by%20ref%29))
  ;[1 1 1] 大破
  (Utilities|Casting|CastToBullet OtherActor
    (:then
      _)
    (:CastFailed
      (Utilities|Casting|CastToSpeedBullet OtherActor)))
  (Effects|SpawnEmitteratLocation "/Game/StarterContent/Particles/P_Explosion_2.P_Explosion_2" (Transformation|GetWorldLocation (Variables|Default|GetBody)) "0, 0, 0" "5.000000,5.000000,5.000000")
  (Actor|DestroyActor))

(event Custom|time
  (bind _returnvalue (Transformation|GetActorLocation))
  (bind _outhit (Collision|LineTraceByChannel _returnvalue (+ _returnvalue (* (Transformation|GetActorUpVector) -1e+03)) "TraceTypeQuery1" false 0 "None"))
  (Rendering|Decal|SpawnDecalatLocation "/Game/Rikuto/Materials/CaterpillarFootprints.CaterpillarFootprints" "120.000000,120.000000,120.000000" (.location _outhit) (Math|Rotator|MakeRotator 0.0 -9e+01 (+ (.yaw (Transformation|GetWorldRotation (Variables|Default|GetBody))) 9e+01)) 0.0))

(event Custom|HItMineEnemy
  ;[1 1 1] 大破
  (Effects|SpawnEmitteratLocation "/Game/StarterContent/Particles/P_Explosion_2.P_Explosion_2" (Transformation|GetWorldLocation (Variables|Default|GetBody)) "0, 0, 0" "5.000000,5.000000,5.000000")
  (Actor|DestroyActor))

(event Collision|EventActorBeginOverlap
  (params (OtherActor :type Actor%20Object%20Reference)))

(event EventTick
  (params (DeltaSeconds :type Float%20%28single-precision%29))
  (bind _returnvalue (Transformation|GetActorRotation))
  (bind _self self)
  (bind _arrow1 (Variables|Default|GetArrow1))
  (bind _enemy1_head (Variables|Default|GetEnemy1_Head))
  (bind _returnvalue_2 (Transformation|GetWorldTransform _arrow1))
  (bind _returnvalue_3 (Utilities|GetDisplayName _self))
  (bind _returnvalue_4 (Transformation|GetWorldLocation _enemy1_head))
  (bind _returnvalue_5 (Utilities|String|RightChop _returnvalue_3 9))
  (bind _returnvalue_6 (+ _returnvalue_4 "0, 0, 0"))
  (bind _returnvalue_7 (Math|Conversions|ToInteger(Byte) _returnvalue_5))
  (bind _returnvalue_8 (- _returnvalue_7 1))
  (bind _returnvalue_9 (Utilities|String|ToString(Integer) _returnvalue_8))
  (bind _returnvalue_10 (Utilities|String|Append "EnemyBullet" _returnvalue_9))
  (bind _returnvalue_11 (Utilities|String|StringToName _returnvalue_10))
  (bind _returnvalue_12 (Actor|GetActorOfClass "/Game/Rikuto/Blueprints/TankGameState.TankGameState_C"))
  (if (Variables|/Game/Rikuto/Blueprints/TankGameState.TankGameState_C|GetPlayerAlive _returnvalue_12) ; プレイヤーが生きているか
    (Transformation|SetWorldRotation (Variables|Default|GetStaticMesh) (Math|Interpolation|RInterpTo (Math|Rotator|MakeRotator (.roll _returnvalue) (.pitch _returnvalue) 0.0) (Math|Rotator|MakeRotator 0.0 0.0 (.yaw (Math|Rotator|FindLookatRotation (Transformation|GetActorLocation) (Transformation|GetActorLocation (Variables|Default|GetPlayer))))) (Utilities|Time|GetWorldDeltaSeconds) 0.0) false false) ; プレイヤーを見る
    ;[1 1 1] 首振り
    (bind _float (Timeline|タイムライン_0 Play)
      (:Update
        (Transformation|SetRelativeRotation (Variables|Default|GetEnemy1_Head) (Math|Rotator|MakeRotator 0.0 0.0 _float) false false)
        (bind (_outhit _returnvalue_13) (Collision|LineTraceByChannel _returnvalue_6 (+ _returnvalue_6 (* (Math|Vector|RotateVectorAroundAxis (Math|Vector|GetForwardVector _enemy1_head) (Variables|Default|GetCurrentAngle) "0.000000,0.000000,1.000000") (Variables|Default|GetDistance))) "TraceTypeQuery1" false 0 "ForOneFrame"))
        (if _returnvalue_13 ; プレイヤーTag持っているか
          (if (Actor|ActorHasTag (.HitActor (Collision|BreakHitResult _outhit)) "Player") ; トレースがプレイヤーに当たっているか
            (if (not (Variables|Default|GetIs%20Stop%20Motion)) ; ストップモーション
              (bind _returnvalue_14 (Actor|GetActorOfClass "/Game/Rikuto/Blueprints/TankGameState.TankGameState_C"))
              (if (> 2 (Utilities|Array|Get(acopy) (Variables|/Game/Rikuto/Blueprints/TankGameState.TankGameState_C|GetEnemyBulletArray _returnvalue_14) _returnvalue_8))
                (Utilities|Array|SetArrayElem (Variables|/Game/Rikuto/Blueprints/TankGameState.TankGameState_C|GetEnemyBulletArray _returnvalue_14) _returnvalue_8 (+ (Utilities|Array|Get(acopy) (Variables|/Game/Rikuto/Blueprints/TankGameState.TankGameState_C|GetEnemyBulletArray _returnvalue_14) _returnvalue_8) 1))
                (if (== (Variables|Default|GetKindofTank) 1) ; タンクが緑なら
                  (bind _returnvalue_15 (Game|SpawnActorfromClass "/Game/kaito/SpeedBullet.SpeedBullet_C" _returnvalue_2 "Undefined" 0 0)) ; 早い球
                  (Utilities|Array|Add (Variables|/Script/Engine.Actor|GetTags _returnvalue_15) _returnvalue_11)
                  (else
                    (bind _returnvalue_16 (Game|SpawnActorfromClass "/Game/kaito/Bullet.Bullet_C" _returnvalue_2 "Undefined" 0 0)) ; 普通の弾
                    (Utilities|Array|Add (Variables|/Script/Engine.Actor|GetTags _returnvalue_16) _returnvalue_11)))
                (Variables|Default|SetIs%20Stop%20Motion true)
                (Utilities|FlowControl|Delay 3.0) ; 0.2秒後
                (Variables|Default|SetIs%20Stop%20Motion false)))))))))

(event EventBeginPlay
  (bind _returnvalue (Actor|GetActorOfClass "/Game/Rikuto/Blueprints/Player.Player_C"))
  (Variables|Default|SetPlayer _returnvalue)
  (Utilities|Time|SetTimerbyEvent (delegate Custom|time) 0.2 true))

(event Input|MouseEvents|RightMouseButton
  (params (Key :type Key%20Structure :default "None"))
  (:Pressed
    (Development|PrintString "Hello" :!label _label))
  (:Released
    (goto _label)))

(event Input|KeyboardEvents|1
  (params (Key :type Key%20Structure :default "None"))
  (:Pressed
    (Development|PrintString "Hello" :!label _label))
  (:Released
    (goto _label)))

(event Input|KeyboardEvents|M
  (params (Key :type Key%20Structure :default "None"))
  (:Pressed
    (Development|PrintString "Hello" :!label _label))
  (:Released
    (goto _label)))

(fn ConstructionScript
  (switch int (Variables|Default|GetKindofTank) ; 0 : 黒  1 : 緑
    (:Default
      (Variables|Default|SetAIControllerClass 0))
    (:0
      (Components|StaticMesh|SetStaticMesh (Variables|Default|GetBody) "/Game/Rikuto/_GENERATED/rikut/Enemy2_body.Enemy2_Body")
      (Components|StaticMesh|SetStaticMesh (Variables|Default|GetEnemy1_Head) "/Game/Rikuto/_GENERATED/rikut/Enemy2_Head.Enemy2_Head")
      (Variables|Default|SetAIControllerClass "/Game/daisuke/BP/AI_Con.AI_Con_C"))
    (:1
      (Components|StaticMesh|SetStaticMesh (Variables|Default|GetBody) "/Game/Rikuto/_GENERATED/rikut/Enemy3_Body.Enemy3_Body")
      (Components|StaticMesh|SetStaticMesh (Variables|Default|GetEnemy1_Head) "/Game/Rikuto/_GENERATED/rikut/Enemy3_Head.Enemy3_Head")
      (Variables|Default|SetAIControllerClass "/Game/daisuke/BP/AI_Con.AI_Con_C")
      (Actor|GetActorOfClass "/Game/kaito/Bullet.Bullet_C"))))

(fn Trace
  (bind _output_get (Variables|Default|SetLast%20Index (Math|Float|Ceil (/ (* (Variables|Default|GetAngle) 2.0) (Variables|Default|GetSpacingAngle))))) ; トレースの数
  (Variables|Default|SetSpacingAngle (/ (* (Variables|Default|GetAngle) 2.0) (Math|Conversions|ToFloat(Integer) _output_get))))