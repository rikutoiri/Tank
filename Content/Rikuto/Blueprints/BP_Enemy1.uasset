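; BP_Enemy1 is an enemy that turns toward the Player and shoots when it spots them.
; Tick interpolates the mesh's rotation toward the player and plays the HeadMove timeline to yaw the head.
; Each timeline update line-traces from the head and spawns a Bullet at the Arrow on hitting a "Player"-tagged actor.
; BeginPlay computes fan-trace spacing via Tlece, but the fan loop and counter-gated firing are disconnected.
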(event Collision|EventActorBeginOverlap
  (params (OtherActor :type Actor%20Object%20Reference)))

(event EventTick
  (params (DeltaSeconds :type Float%20%28single-precision%29))
  (bind _returnvalue (Transformation|GetActorRotation))
  (bind _enemy1_head (Variables|Default|GetEnemy1_Head))
  (bind _returnvalue_2 (Transformation|GetWorldLocation _enemy1_head))
  (bind _returnvalue_3 (+ _returnvalue_2 "0, 0, 0"))
  (bind _returnvalue_4 (Actor|GetActorOfClass "/Game/Rikuto/Blueprints/Player.Player_C"))
  (Variables|Default|SetPlayer _returnvalue_4)
  (Transformation|SetRelativeRotation (Variables|Default|GetStaticMesh) (Math|Interpolation|RInterpTo (Math|Rotator|MakeRotator (.roll _returnvalue) (.pitch _returnvalue) 0.0) (Math|Rotator|MakeRotator 0.0 0.0 (.yaw (Math|Rotator|FindLookatRotation (Transformation|GetActorLocation) (Transformation|GetActorLocation (Variables|Default|GetPlayer))))) (Utilities|Time|GetWorldDeltaSeconds) 0.0) false false)
  (bind _float (Timeline|HeadMove Play)
    (:Update
      (Transformation|SetRelativeRotation (Variables|Default|GetEnemy1_Head) (Math|Rotator|MakeRotator 0.0 0.0 _float) false false)
      (bind _outhit (Collision|LineTraceByChannel _returnvalue_3 (+ _returnvalue_3 (* (Math|Vector|RotateVectorAroundAxis (Math|Vector|GetForwardVector _enemy1_head) (Variables|Default|GetCurrentAngle) "0.000000,0.000000,1.000000") (Variables|Default|GetDistance))) "TraceTypeQuery1" false 0 "ForOneFrame"))
      (if true ; プレイヤーTag持っているか
        (if (Actor|ActorHasTag (.HitActor (Collision|BreakHitResult _outhit)) "Player") ; トレースがプレイヤーに当たっているか
          (Game|SpawnActorfromClass "/Game/kaito/Bullet.Bullet_C" (Transformation|GetWorldTransform (Variables|Default|GetArrow)) "Undefined" 0 0))))))

(event EventBeginPlay
  (CallFunction|Tlece))

(fn ConstructionScript)

(fn Tlece
  (bind _output_get (Variables|Default|SetLast%20Index (Math|Float|Ceil (/ (* (Variables|Default|GetAngle) 2.0) (Variables|Default|GetSpacingAngle))))) ; トレースの数
  (Variables|Default|SetSpacingAngle (/ (* (Variables|Default|GetAngle) 2.0) (Math|Conversions|ToFloat(Integer) _output_get))))