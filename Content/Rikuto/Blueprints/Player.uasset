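; Player tank pawn for a top-down tank game, with movement, cursor-aimed turret, shooting and mine laying.
; Tick rotates the body toward input, moves it with sweeps that slide along obstacles, and turns the head to the cursor.
; Left click fires tagged bullets capped through TankGameState, pausing movement briefly; right click lays a limited number of mines.
; A looping timer stamps track decals while alive, bullet hits spawn explosions, and Space prints enemy bullets.
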(event OnComponentHit(PlayerBody)
  (params (HitComponent :type Primitive%20Component%20Object%20Reference) (OtherActor :type Actor%20Object%20Reference) (OtherComp :type Primitive%20Component%20Object%20Reference) (NormalImpulse :type Vector :default "0, 0, 0") (Hit :type Hit%20Result%20Structure%20%28by%20ref%29))
  (Utilities|Casting|CastToBullet OtherActor)
  (Effects|SpawnEmitteratLocation "/Game/StarterContent/Particles/P_Explosion_2.P_Explosion_2" (Transformation|GetWorldLocation (Variables|Default|GetPlayerBody)) "0, 0, 0" "5.000000,5.000000,5.000000"))

(event Custom|time
  (bind _returnvalue (Transformation|GetActorLocation))
  (bind _returnvalue_2 (Actor|GetActorOfClass "/Game/Rikuto/Blueprints/TankGameState.TankGameState_C"))
  (if (Variables|/Game/Rikuto/Blueprints/TankGameState.TankGameState_C|GetPlayerAlive _returnvalue_2)
    (bind _outhit (Collision|LineTraceByChannel _returnvalue (+ _returnvalue (* (Transformation|GetActorUpVector) -1e+03)) "TraceTypeQuery1" false 0 "None"))
    (Rendering|Decal|SpawnDecalatLocation "/Game/Rikuto/Materials/CaterpillarFootprints.CaterpillarFootprints" "120.000000,120.000000,120.000000" (.location _outhit) (Math|Rotator|MakeRotator 0.0 -9e+01 (+ (.yaw (Transformation|GetWorldRotation (Variables|Default|GetPlayerBody))) 9e+01)) 0.0)))

(event EventBeginPlay
  (Utilities|Time|SetTimerbyEvent (delegate Custom|time) 0.2 true))

(event EventTick
  (params (DeltaSeconds :type Float%20%28single-precision%29))
  (bind _returnvalue (Transformation|GetActorRotation))
  (bind _returnvalue_2 (Input|AxisValues|GetMoveForward))
  (bind _returnvalue_3 (Input|AxisValues|GetMoveRight))
  (bind _movementspeed (Variables|GamePlay|GetMovementSpeed))
  (bind _returnvalue_4 (Math|Vector|MakeVector _returnvalue_2 _returnvalue_3 0.0))
  (bind _returnvalue_5 (* DeltaSeconds _movementspeed))
  (bind _returnvalue_6 (Math|Vector|ClampVectorSize _returnvalue_4 0.0 1.0))
  (bind _returnvalue_7 (* _returnvalue_6 _returnvalue_5))
  (Utilities|FlowControl|Sequence
    (:then_0
      ;[1 1 1] 移動と回転の処理
      (if (not (Variables|Default|GetIsStopMotion)) ; ストップモーション
        (if (> (Math|Vector|VectorLength _returnvalue_7) 0.0)
          (Transformation|SetWorldRotation (Variables|Default|GetPlayerBody) (Math|Conversions|RotationFromXVector _returnvalue_7) false false)
          (bind _sweephitresult (Transformation|AddActorWorldOffset _returnvalue_7 true))
          ;[1 1 1] ポーンがレベル内のアクターとどのように衝突するかを処理する
          (if (.bBlockingHit (Collision|BreakHitResult _sweephitresult))
            (Transformation|AddActorWorldOffset (* (Math|Vector|ProjectVectorontoPlane _returnvalue_7 (Math|Vector|Normalize (Math|Vector|MakeVector (.X (Math|Vector|BreakVector (.Normal (Collision|BreakHitResult _sweephitresult)))) (.Y (Math|Vector|BreakVector (.Normal (Collision|BreakHitResult _sweephitresult)))) 0.0))) (- 1.0 (.Time (Collision|BreakHitResult _sweephitresult)))) true)))))
    (:then_1
      ;[1 1 1] 砲台の向き
      (Transformation|SetWorldRotation (Variables|Default|GetPlayerHead) (Math|Rotator|MakeRotator (.roll _returnvalue) (.pitch _returnvalue) (.yaw (Math|Rotator|FindLookatRotation (Transformation|GetActorLocation) (.Location (Collision|BreakHitResult (.HitResult (Game|Player|GetHitResultUnderCursorbyChannel (Game|GetPlayerController 0) "TraceTypeQuery1" true))))))) false false))))

(event Input|MouseEvents|LeftMouseButton
  (params (Key :type Key%20Structure :default "None"))
  (:Pressed
    (if (not (Variables|Default|GetIsStopMotion)) ; ストップモーション
      (Pawn|SpawnDefaultController)
      ;[1 1 1] 弾が5発まで撃てる
      (bind _returnvalue (Actor|GetActorOfClass "/Game/Rikuto/Blueprints/TankGameState.TankGameState_C"))
      (if (> 5 (Variables|/Game/Rikuto/Blueprints/TankGameState.TankGameState_C|GetPlayerBulletCnt _returnvalue))
        (bind _result (Math|Integer|IncrementInt (Variables|/Game/Rikuto/Blueprints/TankGameState.TankGameState_C|GetPlayerBulletCnt _returnvalue))
          (:%20%20
            (Variables|/Game/Rikuto/Blueprints/TankGameState.TankGameState_C|SetPlayerBulletCnt _returnvalue _result)
            ;[1 1 1] 敵の弾か自分の弾か判断するためスポーンした弾に”PlayerBullet”のタグをつける
            (bind _returnvalue_2 (Game|SpawnActorfromClass "/Game/kaito/Bullet.Bullet_C" (Transformation|GetWorldTransform (Variables|Default|GetArrow)) "Undefined" 0 0))
            (Utilities|Array|Add (Variables|/Script/Engine.Actor|GetTags _returnvalue_2) "PlayerBullet")
            (Variables|Default|SetIsStopMotion true) ; 弾を撃つと動きを止める
            (Utilities|FlowControl|Delay 0.15) ; 0.2秒後
            (Variables|Default|SetIsStopMotion false) ; 動けるようになる
          ))))))

(event Input|KeyboardEvents|SpaceBar
  (params (Key :type Key%20Structure :default "None"))
  (:Pressed
    (bind _returnvalue (Actor|GetActorOfClass "/Game/Rikuto/Blueprints/TankGameState.TankGameState_C"))
    (for _array_element (Variables|/Game/Rikuto/Blueprints/TankGameState.TankGameState_C|GetEnemyBulletArray _returnvalue)
      (Development|PrintString (Utilities|String|ToString(Integer) _array_element)))))

(event Input|MouseEvents|RightMouseButton
  (params (Key :type Key%20Structure :default "None"))
  (:Pressed
    (Pawn|SpawnDefaultController)
    (bind _outactors (Actor|GetAllActorsOfClass "/Game/kaito/mine.mine_C"))
    (if (> 2 (Utilities|Array|Length _outactors))
      (Game|SpawnActorfromClass "/Game/kaito/mine.mine_C" (Transformation|GetWorldTransform (Variables|Default|GetPlayerBody)) "Undefined" 0 0))))

(fn ConstructionScript)