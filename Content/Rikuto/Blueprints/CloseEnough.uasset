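; CloseEnough is a behavior tree decorator for Enemy1_controller that decides when movement toward the followed target should end.
; It measures the straight-line distance from the controlled pawn to the TargetToFollow blackboard actor.
; The condition passes while that distance is at least AcceptableDistance, so despite the name it is true when the enemy is not yet close enough.
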(fn PerformConditionCheck
  (params (OwnerActor :type Actor%20Object%20Reference))
  ;[1 1 1] ターゲット方向への移動終了判定
  (bind _asenemy_1_controller (Utilities|Casting|CastToEnemy1_controller OwnerActor))
  (Variables|Default|SetEnemyController _asenemy_1_controller)
  (return (>= (Math|Vector|VectorLength (- (Transformation|GetActorLocation (AI|BehaviorTree|GetBlackboardValueasActor (Variables|Default|GetTargetToFollow))) (Transformation|GetActorLocation (Pawn|GetControlledPawn (Variables|Default|GetEnemyController))))) (Variables|Default|GetAcceptableDistance))))